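; HealthComponent is an actor component that tracks health for a BP_Char_Base character and signals its death.
; On BeginPlay it casts its owner, binds to the owner's OnTakeAnyDamage event and fills current health to maximum.
; Each hit subtracts damage, refreshes the owner's healthbar widget and calls OnDeathMessage on the owner when health reaches zero or below.
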(event Custom|OnTakeAnyDamage
  (params (DamagedActor :type Actor%20Object%20Reference) (Damage :type Float%20%28single-precision%29) (DamageType :type Damage%20Type%20Object%20Reference) (InstigatedBy :type Controller%20Object%20Reference) (DamageCauser :type Actor%20Object%20Reference))
  ;[1 1 1] Apply Damage and check if the character died
  (bind _output_get (Variables|Default|SetCurrent%20Health (- (Variables|Default|GetCurrent%20Health) Damage)))
  (Default|UpdateHealthbar (Variables|/Game/Blueprints/Characters/Player/BP_Char_Base.BP_Char_Base_C|GetHealthbarWidget (Variables|Default|GetOwnerRef)) _output_get (Variables|Default|GetMax%20Health))
  (if (<= _output_get 0.0)
    (Class|HealthInterface|OnDeath(Message) (Variables|Default|GetOwnerRef))))

(event EventBeginPlay
  ;[1 1 1] Setup
  (bind _asbp_char_base (Utilities|Casting|CastToBP_Char_Base (Components|GetOwner)))
  (bind _output_get (Variables|Default|SetOwnerRef _asbp_char_base))
  (EventDispatchers|BindEventtoOnTakeAnyDamage _output_get (EventDispatchers|CreateEvent :!event Custom|OnTakeAnyDamage))
  (Variables|Default|SetCurrent%20Health (Variables|Default|GetMax%20Health)))