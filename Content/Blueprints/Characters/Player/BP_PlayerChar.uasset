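; Player character Blueprint that shows the cell UI, applies stored morph target values to the mesh and displays a cursor decal in the world.
; On BeginPlay it adds WBP_CellUI to the viewport, then copies each MorphValues entry from RegularGameInstance onto player 0's character mesh.
; Each Tick it moves CursorDecal to the Visibility trace hit under the mouse, oriented along the surface's impact normal.
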(event EventBeginPlay
  (|CallParentFunction)
  (bind _returnvalue (UserInterface|CreateWidget "/Game/Blueprints/Widgets/WBP_CellUI.WBP_CellUI_C"))
  (UserInterface|Viewport|AddtoViewport _returnvalue 0)
  (bind _asregular_game_instance (Utilities|Casting|CastToRegularGameInstance (Game|GetGameInstance)))
  (bind _keys (Utilities|Map|Keys (Variables|/Game/Blueprints/Gamemode/RegularGameInstance.RegularGameInstance_C|GetMorph%20Values _asregular_game_instance)))
  (for _array_element _keys
    (Components|SkeletalMesh|SetMorphTarget (Variables|/Script/Engine.Character|GetMesh (Game|GetPlayerCharacter 0)) _array_element (.Value (Utilities|Map|Find (Variables|/Game/Blueprints/Gamemode/RegularGameInstance.RegularGameInstance_C|GetMorph%20Values _asregular_game_instance) _array_element)) true)))

(event EventTick
  (params (DeltaSeconds :type Float%20%28single-precision%29))
  (bind _returnvalue (Game|GetPlayerController 0))
  (bind _hitresult (Game|Player|GetHitResultUnderCursorbyChannel _returnvalue "TraceTypeQuery1" true))
  (bind (_bblockinghit _binitialoverlap _time _distance _location _impactpoint _normal _impactnormal) (Collision|BreakHitResult _hitresult))
  (Transformation|SetWorldLocationAndRotation (Variables|Default|GetCursorDecal) _location (Math|Rotator|MakeRotationfromAxes _impactnormal "0, 0, 0" "0, 0, 0") false false))

(fn ConstructionScript
  (|CallParentFunction))