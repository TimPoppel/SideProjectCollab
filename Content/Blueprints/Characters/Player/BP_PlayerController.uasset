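; Player controller that drives click-and-hold movement of the BP_PlayerChar pawn toward the cursor.
; Holding SetDestination opens a gate on Tick, which runs a visibility trace under the cursor each frame until release.
; If the hit is at least MinClickDistance away, it calls SimpleMoveToLocation and snaps the character mesh's world yaw to face that point, leaving pitch and roll unchanged.
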(event EventTick
  (params (DeltaSeconds :type Float%20%28single-precision%29))
  (bind _hitresult (Game|Player|GetHitResultUnderCursorbyChannel "TraceTypeQuery1" true))
  (bind _location (Collision|BreakHitResult _hitresult))
  ;[1 1 1] Move and Rotate Player
  (Utilities|FlowControl|Gate true
    (:Exit
      (bind _asbp_player_char (Utilities|Casting|CastToBP_PlayerChar (Pawn|GetControlledPawn)))
      (bind _output_get (Variables|Default|SetCharRef _asbp_player_char))
      (if (>= (Math|Vector|VectorLength (- (Transformation|GetActorLocation _output_get) _location)) (Variables|Default|GetMinClickDistance))
        (AI|Navigation|SimpleMovetoLocation self _location)
        ;;[1 1 1] Set Mesh Rotation
        (Transformation|SetWorldRotation (Variables|/Script/Engine.Character|GetMesh (Variables|Default|GetCharRef)) (Math|Rotator|MakeRotator (.roll (Transformation|GetWorldRotation (Variables|/Script/Engine.Character|GetMesh (Variables|Default|GetCharRef)))) (.pitch (Transformation|GetWorldRotation (Variables|/Script/Engine.Character|GetMesh (Variables|Default|GetCharRef)))) (.yaw (Math|Rotator|FindLookatRotation (Transformation|GetActorLocation _output_get) _location))) false false)))))

(event Input|ActionEvents|InputActionSetDestination
  (params (Key :type Key%20Structure :default "None"))
  (bind _hitresult (Game|Player|GetHitResultUnderCursorbyChannel "TraceTypeQuery1" true))
  (bind _location (Collision|BreakHitResult _hitresult))
  ;[1 1 1] Move and Rotate Player
  (:Pressed
    (Utilities|FlowControl|Gate true) ; enters at Open
  )
  (:Released
    (Utilities|FlowControl|Gate true) ; enters at Close
  ))

(fn ConstructionScript)