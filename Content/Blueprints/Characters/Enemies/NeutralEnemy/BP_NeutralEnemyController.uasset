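; AI controller for the neutral enemy that runs its behavior tree and makes it react to food it perceives.
; When AI perception reports food that passes a FoodType check, it writes the sighting and location to the blackboard and snaps the pawn to face it.
; A DoesSeeFood flag ignores further perception updates until the AteFood event clears it and updates the blackboard.
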(event OnTargetPerceptionUpdated(AIPerception)
  (params (Actor :type Actor%20Object%20Reference) (Stimulus :type AI%20Stimulus%20Structure))
  (if (not (Variables|Default|GetDoesSeeFood))
    (bind _asbp_food (Utilities|Casting|CastToBP_Food Actor))
    (if (Variables|/Game/Blueprints/Environment/BP_Food.BP_Food_C|GetFoodType _asbp_food)
      (bind _output_get (Variables|Default|SetDoesSeeFood true))
      (AI|Components|Blackboard|SetValueasBool (AI|GetBlackboard 0) (Utilities|Name|MakeLiteralName "DoesSeeFood") _output_get)
      (AI|Components|Blackboard|SetValueasVector (AI|GetBlackboard 0) (Utilities|Name|MakeLiteralName "FoodLocation") (Transformation|GetActorLocation _asbp_food))
      (Transformation|SetActorRotation (Pawn|GetControlledPawn) (Math|Rotator|FindLookatRotation (Transformation|GetActorLocation (Pawn|GetControlledPawn)) (Transformation|GetActorLocation _asbp_food))))))

(event EventBeginPlay
  (AI|RunBehaviorTree "/Game/Blueprints/Characters/Enemies/NeutralEnemy/AI/BT_NeutralEnemy.BT_NeutralEnemy")
  (bind _asbp_neutral_enemy (Utilities|Casting|CastToBP_NeutralEnemy (Pawn|GetControlledPawn)))
  (Variables|Default|SetControlledPawn _asbp_neutral_enemy))

(event EventTick
  (params (DeltaSeconds :type Float%20%28single-precision%29)))

(event EventAteFood
  ;[0 1 0.8296] Event Ate Food
  (bind _output_get (Variables|Default|SetDoesSeeFood false))
  (AI|Components|Blackboard|SetValueasBool (AI|GetBlackboard 0) (Utilities|Name|MakeLiteralName "DoesSeeFood") _output_get))

(fn ConstructionScript)