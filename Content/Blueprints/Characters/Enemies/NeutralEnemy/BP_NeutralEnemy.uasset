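; BP_NeutralEnemy is a neutral enemy Blueprint that currently only draws a debug visualization of a forward-facing cone.
; Every Tick it rotates the actor's forward vector 45 degrees to either side and draws a short-lived debug line along each direction.
; It contains no AI, detection or combat logic, and its construction script only calls the parent.
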(event EventBeginPlay
  (|CallParentFunction) ; This node is disabled and will not be called.\nDrag off pins to build functionality.
)

(event Collision|EventActorBeginOverlap
  (params (OtherActor :type Actor%20Object%20Reference)))

(event EventTick
  (params (DeltaSeconds :type Float%20%28single-precision%29))
  (bind _returnvalue (Transformation|GetActorForwardVector))
  (Rendering|Debug|DrawDebugLine (Transformation|GetActorLocation) (+ (* (Math|Vector|RotateVector _returnvalue "0,45.000000, 0") 3e+03) (Transformation|GetActorLocation)) "(R=0.090697,G=0.000000,B=1.000000,A=1.000000)" 0.1 0.0)
  (Rendering|Debug|DrawDebugLine (Transformation|GetActorLocation) (+ (* (Math|Vector|RotateVector _returnvalue "0,-45.000000, 0") 3e+03) (Transformation|GetActorLocation)) "(R=0.090697,G=0.000000,B=1.000000,A=1.000000)" 0.1 0.0))

(fn ConstructionScript
  (|CallParentFunction))