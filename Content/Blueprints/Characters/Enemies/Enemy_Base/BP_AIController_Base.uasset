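; Base AI controller for enemies that runs a behavior tree and steers the controlled enemy toward food it perceives.
; On a perception update, if no food is already seen, it filters food actors by the controller's EatType, with Both accepting any food.
; A match writes DoesSeeFood and FoodLocation to the blackboard and snaps the pawn to face it.
; AteFood clears the seen flag so new food can be accepted.
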(event OnTargetPerceptionUpdated(AIPerception)
  (params (Actor :type Actor%20Object%20Reference) (Stimulus :type AI%20Stimulus%20Structure))
  (bind _eattype (Variables|Default|GetEatType))
  (Variables|Default|SetPerceived%20Actor Actor)
  (Utilities|FlowControl|Sequence
    (:then_0
      (if (not (Variables|Default|GetDoesSeeFood))
        (bind _asbp_food (Utilities|Casting|CastToBP_Food (Variables|Default|GetPerceived%20Actor)))
        (switch Utilities|FlowControl|Switch|SwitchonFoodType _eattype
          (:NewEnumerator0
            (if (Utilities|Enum|Equal(Enum) (Variables|/Game/Blueprints/Environment/BP_Food.BP_Food_C|GetFoodTypeEnum _asbp_food) _eattype) :!label _label
              (bind _output_get (Variables|Default|SetDoesSeeFood true :!label _label_2))
              (AI|Components|Blackboard|SetValueasBool (AI|GetBlackboard 0) (Utilities|Name|MakeLiteralName "DoesSeeFood") _output_get)
              (AI|Components|Blackboard|SetValueasVector (AI|GetBlackboard 0) (Utilities|Name|MakeLiteralName "FoodLocation") (Transformation|GetActorLocation (Variables|Default|GetPerceived%20Actor)))
              (Transformation|SetActorRotation (Variables|Default|GetControlled%20Pawn) (Math|Rotator|FindLookatRotation (Transformation|GetActorLocation (Variables|Default|GetControlled%20Pawn)) (Transformation|GetActorLocation (Variables|Default|GetPerceived%20Actor))))))
          (:NewEnumerator1
            (goto _label))
          (:NewEnumerator2
            (goto _label_2)))))))

(event EventBeginPlay
  (bind _asbp_enemy_base (Utilities|Casting|CastToBP_Enemy_Base (Pawn|GetControlledPawn)))
  (Variables|Default|SetControlled%20Pawn _asbp_enemy_base)
  (AI|RunBehaviorTree (Variables|Default|GetBehaviorTree)))

(event EventTick
  (params (DeltaSeconds :type Float%20%28single-precision%29)))

(event EventAteFood
  (bind _output_get (Variables|Default|SetDoesSeeFood false))
  (AI|Components|Blackboard|SetValueasBool (AI|GetBlackboard 0) (Utilities|Name|MakeLiteralName "DoesSeeFood") _output_get))

(fn ConstructionScript)